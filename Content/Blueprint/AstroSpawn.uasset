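; AstroSpawn is a spawner that keeps creating Astro actors at random points inside the bounds of its Box component.
; Tick counts a timer down and, once it drops below minus one, resets it to a random value, giving roughly one to two seconds between spawns.
; Each Astro appears with a random rotation, including roll, and a fixed uniform scale-up.
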(event EventTick
  (params (DeltaSeconds :type Float%20%28single-precision%29))
  (bind _box (Variables|Default|GetBox))
  (bind (_origin _boxextent) (Collision|GetComponentBounds _box))
  (if (< (Variables|Default|GetspawnTimer) -1.0)
    (Variables|Default|SetspawnTimer (Math|Random|RandomFloatinRange 0.0 1.0))
    (Game|SpawnActorfromClass "/Game/Blueprint/Astro.Astro_C" (Math|Transform|MakeTransform (Math|Vector|MakeVector (Math|Random|RandomFloatinRange (- (.x _origin) (.x _boxextent)) (+ (.x _origin) (.x _boxextent))) (Math|Random|RandomFloatinRange (- (.y _origin) (.y _boxextent)) (+ (.y _origin) (.y _boxextent))) (Math|Random|RandomFloatinRange (- (.z _origin) (.z _boxextent)) (+ (.z _origin) (.z _boxextent)))) (Math|Random|RandomRotator true) "5.000000,5.000000,5.000000") "Undefined" 0 0)
    (else
      (Variables|Default|SetspawnTimer (- (Variables|Default|GetspawnTimer) DeltaSeconds)))))

(fn ConstructionScript)