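; NPC actor that runs a countdown until the Ship picks it up.
; Tick drains TimeLeft and shows it as a fraction of a fixed duration on the WBP_NPCBar widget.
; When time runs out, it sets the player character's O2 negative and destroys itself.
; Sphere overlap with the first Ship found in the level sets that ship's PickedUp flag and destroys the NPC.
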(event OnComponentBeginOverlap(Sphere)
  (params (OverlappedComponent :type Primitive%20Component%20Object%20Reference) (OtherActor :type Actor%20Object%20Reference) (OtherComp :type Primitive%20Component%20Object%20Reference) (OtherBodyIndex :type Integer) (bFromSweep :type Boolean) (SweepResult :type Hit%20Result%20Structure%20%28by%20ref%29))
  (bind _outactors (Actor|GetAllActorsOfClass "/Game/Blueprint/Ship.Ship_C"))
  (if (== (Utilities|Array|Get(acopy) _outactors) OtherActor)
    (Variables|/Game/Blueprint/Ship.Ship_C|SetpickedUp (Utilities|Array|Get(acopy) _outactors) true)
    (Actor|DestroyActor)))

(event EventBeginPlay)

(event Collision|EventActorBeginOverlap
  (params (OtherActor :type Actor%20Object%20Reference)))

(event EventTick
  (params (DeltaSeconds :type Float%20%28single-precision%29))
  (bind _output_get (Variables|Default|SettimeLeft (- (Variables|Default|GettimeLeft) (* (Utilities|Time|GetWorldDeltaSeconds) 1.0))))
  (bind _aswbp_npcbar (Utilities|Casting|CastToWBP_NPCBar (UserInterface|GetUserWidgetObject (Variables|Default|GetWidget))))
  (Progress|SetPercent (Variables|/Game/UI/WBP_NPCBar.WBP_NPCBar_C|GetProgressBar_123 _aswbp_npcbar) (/ _output_get 4.2e+02))
  (if (< (Variables|Default|GettimeLeft) 0.0)
    (bind _asthird_person_character (Utilities|Casting|CastToThirdPersonCharacter (Game|GetPlayerCharacter 0)))
    (Variables|/Game/Blueprint/ThirdPersonCharacter.ThirdPersonCharacter_C|Seto2 _asthird_person_character -5e+01)
    (Actor|DestroyActor)))

(fn ConstructionScript)