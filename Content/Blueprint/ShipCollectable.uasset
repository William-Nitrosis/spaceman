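; Ship part pickup that upgrades the ship when any actor overlaps it.
; On overlap it passes its Part to UpdateShip on the first ShipPart actor found in the level, then destroys itself.
; A looping half-second timer, rather than Tick, appears to drive the player distance check for its widget.
; That check shows the widget only while the player is beyond a distance threshold, hiding it up close.
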(event Custom|CheckPlayerInRangeForUI
  (Rendering|SetVisibility (Variables|Default|GetWidget) (< 4e+04 (Math|Float|Absolute(Float) (Math|Vector|VectorLength (- (Transformation|GetActorLocation (Game|GetPlayerCharacter 0)) (Transformation|GetActorLocation))))) false))

(event EventBeginPlay
  (Utilities|Time|SetTimerbyEvent (EventDispatchers|CreateEvent :!event Custom|CheckPlayerInRangeForUI) 0.5 true))

(event Collision|EventActorBeginOverlap
  (params (OtherActor :type Actor%20Object%20Reference))
  (bind _outactors (Actor|GetAllActorsOfClass "/Game/Blueprint/shipPart.shipPart_C"))
  (bind _asship_part (Utilities|Casting|CastToshipPart (Utilities|Array|Get(acopy) _outactors)))
  (Default|UpdateShip _asship_part (Variables|Default|Getpart))
  (Actor|DestroyActor))

(event EventTick
  (params (DeltaSeconds :type Float%20%28single-precision%29)))

(fn ConstructionScript)