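; Hazard volume actor that flags the player character as exposed to cold, heat or radiation while it overlaps the volume.
; A String variable selects the hazard type, and begin and end overlap set and clear the matching InCold, InHot or InRad flag on ThirdPersonCharacter.
; Cold also raises the character's O2Mult during overlap and resets it to normal on exit.
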(event Collision|EventActorBeginOverlap
  (params (OtherActor :type Actor%20Object%20Reference))
  (if (== (Utilities|GetClass OtherActor) "/Game/Blueprint/ThirdPersonCharacter.ThirdPersonCharacter_C")
    (switch string (Variables|Default|Getstring)
      (:cold
        (bind _asthird_person_character (Utilities|Casting|CastToThirdPersonCharacter OtherActor))
        (Variables|/Game/Blueprint/ThirdPersonCharacter.ThirdPersonCharacter_C|Seto2Mult _asthird_person_character 5.0)
        (Variables|/Game/Blueprint/ThirdPersonCharacter.ThirdPersonCharacter_C|SetinCold _asthird_person_character true))
      (:heat
        (bind _asthird_person_character_2 (Utilities|Casting|CastToThirdPersonCharacter OtherActor))
        (Variables|/Game/Blueprint/ThirdPersonCharacter.ThirdPersonCharacter_C|SetinHot _asthird_person_character_2 true))
      (:rad
        (bind _asthird_person_character_3 (Utilities|Casting|CastToThirdPersonCharacter OtherActor))
        (Variables|/Game/Blueprint/ThirdPersonCharacter.ThirdPersonCharacter_C|SetinRad _asthird_person_character_3 true)))))

(event Collision|EventActorEndOverlap
  (params (OtherActor :type Actor%20Object%20Reference))
  (if (== (Utilities|GetClass OtherActor) "/Game/Blueprint/ThirdPersonCharacter.ThirdPersonCharacter_C")
    (switch string (Variables|Default|Getstring)
      (:cold
        (bind _asthird_person_character (Utilities|Casting|CastToThirdPersonCharacter OtherActor))
        (Variables|/Game/Blueprint/ThirdPersonCharacter.ThirdPersonCharacter_C|Seto2Mult _asthird_person_character 1.0)
        (Variables|/Game/Blueprint/ThirdPersonCharacter.ThirdPersonCharacter_C|SetinCold _asthird_person_character false))
      (:heat
        (bind _asthird_person_character_2 (Utilities|Casting|CastToThirdPersonCharacter OtherActor))
        (Variables|/Game/Blueprint/ThirdPersonCharacter.ThirdPersonCharacter_C|SetinHot _asthird_person_character_2 false))
      (:rad
        (bind _asthird_person_character_3 (Utilities|Casting|CastToThirdPersonCharacter OtherActor))
        (Variables|/Game/Blueprint/ThirdPersonCharacter.ThirdPersonCharacter_C|SetinRad _asthird_person_character_3 false)))))

(fn ConstructionScript)