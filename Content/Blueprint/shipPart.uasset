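; Buildable ship actor that stands in for the Ship while the ship is assembled from six parts: four legs, buttons and thrusters.
; BeginPlay hides all parts, then each updateShip call reveals the named part and increments BuildProgress.
; Tick polls that counter and, once all six are counted, enables collision on the first Ship in the level, triggers its Spawn and destroys this actor.
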(event Custom|updateShip
  (params (part :type String))
  (switch string part
    (:leg1
      (Rendering|SetVisibility (Variables|Default|GetLeg1) true false))
    (:leg2
      (Rendering|SetVisibility (Variables|Default|GetLeg2) true false))
    (:leg3
      (Rendering|SetVisibility (Variables|Default|GetLeg3) true false))
    (:leg4
      (Rendering|SetVisibility (Variables|Default|GetLeg4) true false))
    (:buttons
      (Rendering|SetVisibility (Variables|Default|GetButtons) true false))
    (:thrusters
      (Rendering|SetVisibility (Variables|Default|GetThrusters) true false)))
  (Math|Integer|IncrementInt (Variables|Default|GetbuildProgress)))

(event EventBeginPlay
  (Rendering|SetVisibility (Variables|Default|GetButtons) false false)
  (Variables|Default|SetbuildProgress 0))

(event Collision|EventActorBeginOverlap
  (params (OtherActor :type Actor%20Object%20Reference)))

(event EventTick
  (params (DeltaSeconds :type Float%20%28single-precision%29))
  (if (== (Variables|Default|GetbuildProgress) 6)
    (bind _outactors (Actor|GetAllActorsOfClass "/Game/Blueprint/Ship.Ship_C"))
    (bind _asship (Utilities|Casting|CastToShip (Utilities|Array|Get(acopy) _outactors)))
    (Collision|SetCollisionEnabled (Variables|/Game/Blueprint/Ship.Ship_C|GetStaticMesh _asship) "QueryAndPhysics")
    (Variables|/Game/Blueprint/Ship.Ship_C|SettoSpawn _asship true)
    (Default|Spawn _asship)
    (Actor|DestroyActor)))

(fn ConstructionScript)