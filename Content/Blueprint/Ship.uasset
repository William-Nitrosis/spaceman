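; Pilotable ship pawn that the player takes over from the third-person character.
; It starts hidden with mesh collision off, and a Spawn event applies the ToSpawn flag, which is never set true here, to mesh visibility.
; When ToSpawn is true, a character overlapping the box triggers one-time possession and is destroyed.
; Input axes drive yaw and pitch, camera-relative planar movement, and vertical movement along the mesh's up vector.
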(event OnComponentBeginOverlap(Box)
  (params (OverlappedComponent :type Primitive%20Component%20Object%20Reference) (OtherActor :type Actor%20Object%20Reference) (OtherComp :type Primitive%20Component%20Object%20Reference) (OtherBodyIndex :type Integer) (bFromSweep :type Boolean) (SweepResult :type Hit%20Result%20Structure%20%28by%20ref%29))
  (bind _asthird_person_character (Utilities|Casting|CastToThirdPersonCharacter OtherActor))
  (if (Variables|Default|GettoSpawn)
    (Utilities|FlowControl|DoOnce false
      (:Completed
        (Pawn|Possess (Game|GetPlayerController 0) self)
        (Actor|DestroyActor _asthird_person_character)))))

(event Custom|Spawn
  (Rendering|SetVisibility (Variables|Default|GetStaticMesh) (Variables|Default|GettoSpawn) false))

(event EventTick
  (params (DeltaSeconds :type Float%20%28single-precision%29)))

(event EventBeginPlay
  (bind _staticmesh (Variables|Default|GetStaticMesh))
  (bind _output_get (Variables|Default|SettoSpawn false))
  (Rendering|SetVisibility _staticmesh _output_get false)
  (Collision|SetCollisionEnabled _staticmesh "NoCollision"))

(event Input|AxisEvents|InputAxisLookUp
  (params (AxisValue :type Float%20%28single-precision%29))
  (Pawn|Input|AddControllerPitchInput AxisValue))

(event Input|AxisEvents|InputAxisTurn
  (params (AxisValue :type Float%20%28single-precision%29))
  (Pawn|Input|AddControllerYawInput AxisValue))

(event Input|AxisEvents|InputAxisVertMovement
  (params (AxisValue :type Float%20%28single-precision%29))
  (Pawn|Input|AddMovementInput (Math|Vector|GetUpVector (Variables|Default|GetStaticMesh)) AxisValue false))

(event Input|AxisEvents|InputAxisMoveForward
  (params (AxisValue :type Float%20%28single-precision%29))
  (Pawn|Input|AddMovementInput (Math|Vector|GetForwardVector (Variables|Default|GetCamera)) AxisValue false))

(event Input|AxisEvents|InputAxisMoveRight
  (params (AxisValue :type Float%20%28single-precision%29))
  (Pawn|Input|AddMovementInput (Math|Vector|GetRightVector (Variables|Default|GetCamera)) AxisValue false))

(fn ConstructionScript)