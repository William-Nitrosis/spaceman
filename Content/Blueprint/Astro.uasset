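; Astro is an asteroid actor that drifts and tumbles through the world, then destroys itself once its age exceeds Lifetime.
; The construction script picks a random asteroid mesh, though RandomInteger(5) never reaches the sixth.
; BeginPlay applies a large impulse in a random direction and stores a separate random vector.
; Tick turns that vector into a small rotation added every frame, so spin speed depends on frame rate.
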(event EventBeginPlay
  (bind _returnvalue (Math|Random|RandomFloatinRange -1.0 1.0))
  (bind _returnvalue_2 (Math|Random|RandomFloatinRange -1.0 1.0))
  (bind _returnvalue_3 (Math|Random|RandomFloatinRange -1.0 1.0))
  (bind _returnvalue_4 (Math|Vector|MakeVector _returnvalue _returnvalue_2 _returnvalue_3))
  (Physics|AddImpulse (Variables|Default|GetStaticMesh) (* _returnvalue_4 29999998.0) "None" false)
  (Variables|Default|SetvelocityVector _returnvalue_4))

(event EventTick
  (params (DeltaSeconds :type Float%20%28single-precision%29))
  (Transformation|AddRelativeRotation (Variables|Default|GetStaticMesh) (* (Math|Conversions|RotationFromXVector (/ (Variables|Default|GetvelocityVector) DeltaSeconds)) 0.001) false false)
  (if (> (Actor|GetGameTimeSinceCreation) (Variables|Default|GetLifetime))
    (Actor|DestroyActor)))

(fn ConstructionScript
  (bind _staticmesh (Variables|Default|GetStaticMesh))
  (switch int (Math|Random|RandomInteger 5)
    (:0
      (Components|StaticMesh|SetStaticMesh _staticmesh "/Game/Geometry/Meshes/Astroids_001.Astroids_001"))
    (:1
      (Components|StaticMesh|SetStaticMesh _staticmesh "/Game/Geometry/Meshes/Astroids_002.Astroids_002"))
    (:2
      (Components|StaticMesh|SetStaticMesh _staticmesh "/Game/Geometry/Meshes/Astroids_003.Astroids_003"))
    (:3
      (Components|StaticMesh|SetStaticMesh _staticmesh "/Game/Geometry/Meshes/Astroids_004.Astroids_004"))
    (:4
      (Components|StaticMesh|SetStaticMesh _staticmesh "/Game/Geometry/Meshes/Astroids_005.Astroids_005"))
    (:5
      (Components|StaticMesh|SetStaticMesh _staticmesh "/Game/Geometry/Meshes/Astroids_006.Astroids_006"))))