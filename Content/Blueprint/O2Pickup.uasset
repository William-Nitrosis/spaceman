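; O2Pickup is an oxygen pickup that calls O2Refill on an overlapping ThirdPersonCharacter and destroys itself.
; On spawn the mesh gets a random impulse and tumbles each tick along a random vector.
; A looping timer is set up, and a range-check event shows the widget only when the player is beyond a near threshold but within UIViewDist.
; Once its Lifetime expires, it spawns an air explosion emitter and destroys itself.
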(event OnComponentBeginOverlap(Capsule)
  (params (OverlappedComponent :type Primitive%20Component%20Object%20Reference) (OtherActor :type Actor%20Object%20Reference) (OtherComp :type Primitive%20Component%20Object%20Reference) (OtherBodyIndex :type Integer) (bFromSweep :type Boolean) (SweepResult :type Hit%20Result%20Structure%20%28by%20ref%29))
  (bind _asthird_person_character (Utilities|Casting|CastToThirdPersonCharacter OtherActor))
  (Default|O2Refill _asthird_person_character)
  (Actor|DestroyActor))

(event Custom|CheckPlayerInRangeForUI
  (bind _returnvalue (Transformation|GetActorLocation))
  (bind _returnvalue_2 (Game|GetPlayerCharacter 0))
  (bind _returnvalue_3 (Transformation|GetActorLocation _returnvalue_2))
  (bind _returnvalue_4 (- _returnvalue_3 _returnvalue))
  (bind _returnvalue_5 (Math|Vector|VectorLength _returnvalue_4))
  (bind _returnvalue_6 (Math|Float|Absolute(Float) _returnvalue_5))
  (Rendering|SetVisibility (Variables|Default|GetWidget) (and (< _returnvalue_6 (Variables|Default|GetUIViewDist)) (< 5e+03 _returnvalue_6)) false))

(event EventBeginPlay
  (bind _returnvalue (Math|Random|RandomFloatinRange -1.0 1.0))
  (bind _returnvalue_2 (Math|Random|RandomFloatinRange -1.0 1.0))
  (bind _returnvalue_3 (Math|Random|RandomFloatinRange -1.0 1.0))
  (bind _returnvalue_4 (Math|Vector|MakeVector _returnvalue _returnvalue_2 _returnvalue_3))
  (Physics|AddImpulse (Variables|Default|GetStaticMesh) (* _returnvalue_4 3e+03) "None" false)
  (Variables|Default|SetvelocityVector _returnvalue_4)
  (Utilities|Time|SetTimerbyEvent (EventDispatchers|CreateEvent :!event Custom|CheckPlayerInRangeForUI) 0.5 true))

(event EventTick
  (params (DeltaSeconds :type Float%20%28single-precision%29))
  (Transformation|AddRelativeRotation (Variables|Default|GetStaticMesh) (* (Math|Conversions|RotationFromXVector (/ (Variables|Default|GetvelocityVector) DeltaSeconds)) 0.01) false false)
  (if (> (Actor|GetGameTimeSinceCreation) (Variables|Default|GetLifetime))
    (Effects|SpawnEmitteratLocation "/Game/Part/AirExplosion.AirExplosion" (Transformation|GetActorLocation))
    (Actor|DestroyActor)))

(fn ConstructionScript)